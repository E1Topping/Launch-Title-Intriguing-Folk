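; Pickup actor for the fourth note in the detective game, collected with the Interact input.
; Its box overlap with the Detective_2D_Character enables player input and opens a Gate, and leaving disables both.
; Pressing Interact through the open gate sets HasNote4 on the character, notifies its Notebook via GottedNote4 and destroys the actor.
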(event `InputAction|Interact`
  (params (Key :type "Key Structure"))
  (:`Pressed`
    (`/Engine/EditorBlueprintResources/StandardMacros.Gate` true :!label _label
      (:`Exit`
        (set `/Game/Sophie/Detective_2D_Character.has_note_4` true (stale `self.Box.OnComponentBeginOverlap` _asdetective_2d_character))
        (`/Game/Sophie/Notebook.gotted note 4` (`/Game/Sophie/Detective_2D_Character.notebook` (stale `self.Box.OnComponentBeginOverlap` _asdetective_2d_character)))
        (`self.K2_DestroyActor`)))))

(event `self.Box.OnComponentBeginOverlap`
  (params (OverlappedComponent :type "PrimitiveComponent Object Reference") (OtherActor :type "Actor Object Reference") (OtherComp :type "PrimitiveComponent Object Reference") (OtherBodyIndex :type Integer) (bFromSweep :type Boolean) (SweepResult :type "HitResult Structure (by ref)"))
  (bind _asdetective_2d_character (cast `/Game/Sophie/Detective_2D_Character` OtherActor))
  (`self.EnableInput` (`GameplayStatics.GetPlayerController` 0))
  (goto _label :!via `Open`))

(event `self.Box.OnComponentEndOverlap`
  (params (OverlappedComponent :type "PrimitiveComponent Object Reference") (OtherActor :type "Actor Object Reference") (OtherComp :type "PrimitiveComponent Object Reference") (OtherBodyIndex :type Integer))
  (cast `/Game/Sophie/Detective_2D_Character` OtherActor)
  (`self.DisableInput` (`GameplayStatics.GetPlayerController` 0))
  (goto _label :!via `Close`))

(fn `UserConstructionScript`)
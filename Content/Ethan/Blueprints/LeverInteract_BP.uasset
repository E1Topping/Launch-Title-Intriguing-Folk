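; LeverInteract_BP is an interactable that plays a sequence through SequncePlayer when a Detective_2D_Character who has the lever presses Interact.
; Box overlap enables player input and opens a gate for that sequence, and leaving reverses both.
; Without the lever, Interact shows a dialogue widget with its Text for three seconds, skipping creation while one is already showing.
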(event `InputAction|Interact`
  (params (Key :type "Key Structure"))
  (:`Pressed`
    (if (`/Game/Sophie/Detective_2D_Character.has_lever` (stale `self.Box.OnComponentBeginOverlap` _asdetective_2d_character))
      (`/Engine/EditorBlueprintResources/StandardMacros.Gate` true :!label _label
        (:`Exit`
          (`/Game/Sophie/scripted_sequences/play_sequence.PlaySqeunce` (`self.sequncePlayer`))))
      (else
        (`/Engine/EditorBlueprintResources/StandardMacros.IsValid` (`self.dialogue_widget`)
          (:`Is Not Valid`
            (bind _returnvalue (`|CreateWidget` "/Game/Sophie/dialogue/Dialogue_widget.Dialogue_widget_C" (`GameplayStatics.GetPlayerController` 0)))
            (bind _output_get (set `self.Dialogue_Widget` _returnvalue))
            (`UserWidget.AddToViewport` _output_get 0)
            (set `/Game/Sophie/dialogue/Dialogue_widget.Dialogue_text` (`self.text`) (`self.dialogue_widget`))
            (`KismetSystemLibrary.Delay` 3.0)
            (`Widget.RemoveFromParent` (`self.dialogue_widget`))
            (set `self.dialogue_widget` null)))))))

(event `self.Box.OnComponentBeginOverlap`
  (params (OverlappedComponent :type "PrimitiveComponent Object Reference") (OtherActor :type "Actor Object Reference") (OtherComp :type "PrimitiveComponent Object Reference") (OtherBodyIndex :type Integer) (bFromSweep :type Boolean) (SweepResult :type "HitResult Structure (by ref)"))
  (bind _asdetective_2d_character (cast `/Game/Sophie/Detective_2D_Character` OtherActor))
  (`self.EnableInput` (`GameplayStatics.GetPlayerController` 0))
  (goto _label :!via `Open`))

(event `self.Box.OnComponentEndOverlap`
  (params (OverlappedComponent :type "PrimitiveComponent Object Reference") (OtherActor :type "Actor Object Reference") (OtherComp :type "PrimitiveComponent Object Reference") (OtherBodyIndex :type Integer))
  (cast `/Game/Sophie/Detective_2D_Character` OtherActor)
  (`self.DisableInput` (`GameplayStatics.GetPlayerController` 0))
  (goto _label :!via `Close`))

(fn `UserConstructionScript`)
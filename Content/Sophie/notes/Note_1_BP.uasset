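; Pickup actor for the first note, which shows dialogue text and flags HasNote1 on the Detective_2D_Character.
; Box overlap caches the character, enables input and opens a gate; leaving disables input and closes it.
; Interact shows a Dialogue_widget for a fixed delay, then removes it.
; If the gate is still open after the delay, it sets the flag and destroys the note.
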(event `InputAction|Interact`
  (params (Key :type "Key Structure"))
  (:`Pressed`
    (`/Engine/EditorBlueprintResources/StandardMacros.IsValid` (`self.dialoguewidget`)
      (:`Is Not Valid`
        (bind _returnvalue (`|CreateWidget` "/Game/Sophie/dialogue/Dialogue_widget.Dialogue_widget_C"))
        (bind _output_get (set `self.dialoguewidget` _returnvalue))
        (`UserWidget.AddToViewport` _output_get 0)
        (set `/Game/Sophie/dialogue/Dialogue_widget.Dialogue_text` (`self.Dialogue Text`) (`self.dialoguewidget`))
        (`KismetSystemLibrary.Delay` 2.5)
        (`Widget.RemoveFromParent` (`self.dialoguewidget`))
        (set `self.dialoguewidget` null)
        (`/Engine/EditorBlueprintResources/StandardMacros.Gate` true :!label _label
          (:`Exit`
            (set `/Game/Sophie/Detective_2D_Character.has_note_1` true (stale `self.Box.OnComponentBeginOverlap` _asdetective_2d_character))
            (`self.K2_DestroyActor`)))))))

(event `self.Box.OnComponentBeginOverlap`
  (params (OverlappedComponent :type "PrimitiveComponent Object Reference") (OtherActor :type "Actor Object Reference") (OtherComp :type "PrimitiveComponent Object Reference") (OtherBodyIndex :type Integer) (bFromSweep :type Boolean) (SweepResult :type "HitResult Structure (by ref)"))
  (bind _asdetective_2d_character (cast `/Game/Sophie/Detective_2D_Character` OtherActor))
  (`self.EnableInput` (`GameplayStatics.GetPlayerController` 0))
  (goto _label :!via `Open`))

(event `self.Box.OnComponentEndOverlap`
  (params (OverlappedComponent :type "PrimitiveComponent Object Reference") (OtherActor :type "Actor Object Reference") (OtherComp :type "PrimitiveComponent Object Reference") (OtherBodyIndex :type Integer))
  (cast `/Game/Sophie/Detective_2D_Character` OtherActor)
  (`self.DisableInput` (`GameplayStatics.GetPlayerController` 0))
  (goto _label :!via `Close`))

(fn `UserConstructionScript`)
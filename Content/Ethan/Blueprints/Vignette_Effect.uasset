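; Actor Blueprint that temporarily swaps a post process volume's settings for a vignette effect.
; BeginPlay caches the volume's current settings as the default and also assigns the vignette settings.
; The TriggerEffect event applies the vignette settings, waits for the Length duration, then restores the cached defaults.
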(event `self.ReceiveBeginPlay`
  (bind _postporcessvolume (`self.PostPorcessVolume`))
  (bind _output_get (set `PostProcessVolume.Settings` (`PostProcessVolume.Settings` _postporcessvolume) _postporcessvolume))
  (set `self.DefualtSettings` _output_get)
  (set `self.VignetteSettings` (struct)))

(event `Trigger Effect`
  (set `PostProcessVolume.Settings` (`self.VignetteSettings`) (`self.PostPorcessVolume`))
  (`KismetSystemLibrary.Delay` (`self.Length`))
  (set `PostProcessVolume.Settings` (`self.DefualtSettings`) (`self.PostPorcessVolume`)))

(fn `UserConstructionScript`)
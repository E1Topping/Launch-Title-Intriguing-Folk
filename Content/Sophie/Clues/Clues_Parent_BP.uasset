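; Parent Blueprint for clue pickups that the Detective_2D_Character collects by pressing Interact.
; Box overlap with the detective shows a Text prompt, enables player input on the clue and opens a Gate, and leaving reverses all three.
; Pressing Interact while the gate is open sets the detective's Clue1 flag and destroys the clue actor.
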(event `InputAction|Interact`
  (params (Key :type "Key Structure"))
  (:`Pressed`
    (`/Engine/EditorBlueprintResources/StandardMacros.Gate` true :!label _label
      (:`Exit`
        (set `/Game/Sophie/Detective_2D_Character.clue_1` true (stale `self.Box.OnComponentBeginOverlap` _asdetective_2d_character))
        (`self.K2_DestroyActor`)))))

(event `self.Box.OnComponentBeginOverlap`
  (params (OverlappedComponent :type "PrimitiveComponent Object Reference") (OtherActor :type "Actor Object Reference") (OtherComp :type "PrimitiveComponent Object Reference") (OtherBodyIndex :type Integer) (bFromSweep :type Boolean) (SweepResult :type "HitResult Structure (by ref)"))
  (bind _asdetective_2d_character (cast `/Game/Sophie/Detective_2D_Character` OtherActor))
  (`SceneComponent.SetVisibility` (`self.text`) true false)
  (`self.EnableInput` (`GameplayStatics.GetPlayerController` 0))
  (goto _label :!via `Open`))

(event `self.Box.OnComponentEndOverlap`
  (params (OverlappedComponent :type "PrimitiveComponent Object Reference") (OtherActor :type "Actor Object Reference") (OtherComp :type "PrimitiveComponent Object Reference") (OtherBodyIndex :type Integer))
  (cast `/Game/Sophie/Detective_2D_Character` OtherActor)
  (`SceneComponent.SetVisibility` (`self.text`) false false)
  (`self.DisableInput` (`GameplayStatics.GetPlayerController` 0))
  (goto _label :!via `Close`))

(fn `UserConstructionScript`)